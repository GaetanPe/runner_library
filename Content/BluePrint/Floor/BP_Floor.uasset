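; BP_Floor is a floor segment for a runner game that triggers track extension and speeds up the player.
; When its BoxCollision is overlapped, it asks BP_RunnerGM to extend the floor, then multiplies player 0's max walk speed by SpeedGrowth within a clamped range.
; The overlap does not check which actor entered.
; GetAttachPoint exposes the Arrow component's world transform as an attach point.
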(event `self.Box Collision.OnComponentBeginOverlap`
  (params (OverlappedComponent :type "PrimitiveComponent Object Reference") (OtherActor :type "Actor Object Reference") (OtherComp :type "PrimitiveComponent Object Reference") (OtherBodyIndex :type Integer) (bFromSweep :type Boolean) (SweepResult :type "HitResult Structure (by ref)"))
  ;[1 1 1] Extend Floor
  (bind _asbp_runner_gm (cast `/Game/BluePrint/BP_RunnerGM` (`GameplayStatics.GetGameMode`)))
  (`/Game/BluePrint/BP_RunnerGM.ExtendFloor` _asbp_runner_gm)
  ;[1 1 1] Speed Increase
  (bind _asbp_player (cast `/Game/BluePrint/Player/BP_Player` (`GameplayStatics.GetPlayerCharacter` 0)))
  (bind _charactermovement (`Character.CharacterMovement` _asbp_player))
  (set `CharacterMovementComponent.MaxWalkSpeed` (`KismetMathLibrary.FClamp` (* (`CharacterMovementComponent.MaxWalkSpeed` _charactermovement) (`self.SpeedGrowth`)) 600.0 2000.0) _charactermovement))

(fn `GetAttachPoint`
  (returns (ArrowWorldTransform :type "Transform Structure"))
  (return (`SceneComponent.K2_GetComponentToWorld` (`self.Arrow`))))

(fn `UserConstructionScript`)