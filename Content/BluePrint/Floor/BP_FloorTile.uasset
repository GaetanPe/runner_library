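; Floor tile for an endless runner that extends the track and speeds up the player when its box trigger is overlapped.
; Overlap asks BP_RunnerGM to extend the floor and multiplies the player's walk speed by SpeedGrowth within a clamped range.
; Construction builds two rows of arrow spawn points across the lanes.
; SpawnObstacles shuffles them to place random child-actor obstacles, while GetAttachPoint returns the Arrow's world transform.
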(event `self.Box Collision.OnComponentBeginOverlap`
  (params (OverlappedComponent :type "PrimitiveComponent Object Reference") (OtherActor :type "Actor Object Reference") (OtherComp :type "PrimitiveComponent Object Reference") (OtherBodyIndex :type Integer) (bFromSweep :type Boolean) (SweepResult :type "HitResult Structure (by ref)"))
  ;[1 1 1] Extend Floor
  (bind _asbp_runner_gm (cast `/Game/BluePrint/BP_RunnerGM` (`GameplayStatics.GetGameMode`)))
  (`/Game/BluePrint/BP_RunnerGM.ExtendFloor` _asbp_runner_gm)
  ;[1 1 1] Speed Increase
  (bind _asbp_player (cast `/Game/BluePrint/Player/BP_Player` (`GameplayStatics.GetPlayerCharacter` 0)))
  (bind _charactermovement (`Character.CharacterMovement` _asbp_player))
  (set `CharacterMovementComponent.MaxWalkSpeed` (`KismetMathLibrary.FClamp` (* (`CharacterMovementComponent.MaxWalkSpeed` _charactermovement) (`self.SpeedGrowth`)) 600.0 2000.0) _charactermovement))

(fn `GetAttachPoint`
  (returns (ArrowWorldTransform :type "Transform Structure"))
  (return (`SceneComponent.K2_GetComponentToWorld` (`self.Arrow`))))

(fn `SetPawnPoints`
  (for _array_element (`self.Lane Position`)
    (for _index (range 2)
      (bind _returnvalue (`AddComponent|NODE_AddArrowComponent-0` :`RelativeTransform` (`KismetMathLibrary.MakeTransform` (`KismetMathLibrary.MakeVector` (* _index 650.0) _array_element))))
      (`KismetArrayLibrary.Array_Add` (`self.Spawn Points`) (`SceneComponent.K2_GetComponentToWorld` _returnvalue)))))

(fn `Spawn Obstacles`
  (locals (`Ramdom Spawn  Points` :type "Array of Transform Structure"))
  (bind _output_get (set `local.Ramdom Spawn  Points` (`self.Spawn Points`)))
  (`KismetArrayLibrary.Array_Shuffle` _output_get)
  (for _index (range (+ (`KismetMathLibrary.RandomIntegerInRange` 0 2) 1))
    (switch `int` (`KismetMathLibrary.RandomIntegerInRange` 0)
      (:`0`
        (bind _returnvalue (`KismetMathLibrary.MakeRelativeTransform` (`|GetArrayItem` (`local.Ramdom Spawn  Points`) _index) (`self.GetTransform`)))
        (`AddComponent|NODE_AddChildActorComponent-0` :`RelativeTransform` _returnvalue))
      (:`1`
        (`AddComponent|NODE_AddChildActorComponent-1` :`RelativeTransform` _returnvalue)))))

(fn `UserConstructionScript`
  (`self.SetPawnPoints`))