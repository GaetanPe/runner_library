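; Floor tile for an endless runner that populates itself with obstacles, coins and an occasional power-up.
; The construction script builds per-lane spawn points, shuffles them and attaches child actors, adding a power-up when the game mode's FloorCount passes a threshold, then resetting it.
; Overlapping its box makes the game mode extend the floor, slightly raises the player's clamped walk speed and adds multiplier-based points.
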(event `self.Box.OnComponentBeginOverlap`
  (params (OverlappedComponent :type "PrimitiveComponent Object Reference") (OtherActor :type "Actor Object Reference") (OtherComp :type "PrimitiveComponent Object Reference") (OtherBodyIndex :type Integer) (bFromSweep :type Boolean) (SweepResult :type "HitResult Structure (by ref)"))
  ;[1 1 1] Extension des tuiles
  (bind _asbp_runner_game_mode (cast `/Game/Runner/BluePrint/BP_RunnerGameMode` (`GameplayStatics.GetGameMode`)))
  (`/Game/Runner/BluePrint/BP_RunnerGameMode.extend floor` _asbp_runner_game_mode)
  ;[1 1 1] Mise a jour de la vitesse
  (bind _asbp_runner_character (cast `/Game/Runner/BluePrint/Characters/Bp_RunnerCharacter` (`GameplayStatics.GetPlayerCharacter` 0)))
  (bind _charactermovement (`Character.CharacterMovement` _asbp_runner_character))
  (bind _output_get (set `CharacterMovementComponent.MaxWalkSpeed` (`KismetMathLibrary.FClamp` (* (`CharacterMovementComponent.MaxWalkSpeed` _charactermovement) 1.001) 700.0 1500.0) _charactermovement))
  (`KismetSystemLibrary.PrintString` (`KismetStringLibrary.Conv_DoubleToString` _output_get))
  ;[1 1 1] Mise a jour score
  (bind _asbp_runner_game_mode_2 (cast `/Game/Runner/BluePrint/BP_RunnerGameMode` (`GameplayStatics.GetGameMode`)))
  (set `/Game/Runner/BluePrint/BP_RunnerGameMode.CurrentPoints` (+ (* (`/Game/Runner/BluePrint/BP_RunnerGameMode.Points Multi` _asbp_runner_game_mode_2) 1) (`/Game/Runner/BluePrint/BP_RunnerGameMode.CurrentPoints` _asbp_runner_game_mode_2)) _asbp_runner_game_mode_2))

(fn `Coin Spawn Points`
  (for _array_element (`self.Lane Position`)
    (for _index (range 10)
      (bind _returnvalue (`AddComponent|NODE_AddArrowComponent-1` :`RelativeTransform` (`KismetMathLibrary.MakeTransform` (`KismetMathLibrary.MakeVector` (* _index 75.0) _array_element))))
      (`ArrowComponent.SetArrowColor` _returnvalue (struct :`R` 0.024899 :`G` 0.24288 :`B` 1.0 :`A` 1.0))
      (`KismetArrayLibrary.Array_Add` (`self.CSpawn Points`) (`SceneComponent.K2_GetComponentToWorld` _returnvalue)))))

(fn `Get AttachPoint`
  (returns (ReturnValue :type "Transform Structure"))
  (return (`SceneComponent.K2_GetComponentToWorld` (`self.Arrow`))))

(fn `PowerUp_SpawnPoints`
  (for _array_element (`self.Lane Position`)
    (for _index (range 1 3)
      (bind _returnvalue (`AddComponent|NODE_AddArrowComponent-2` :`RelativeTransform` (`KismetMathLibrary.MakeTransform` (`KismetMathLibrary.MakeVector` (* _index 250.0) _array_element))))
      (`ArrowComponent.SetArrowColor` _returnvalue (struct :`R` 0.885734 :`G` 1.0 :`B` 0.249381 :`A` 1.0))
      (`KismetArrayLibrary.Array_Add` (`self.PSpawnPoints`) (`SceneComponent.K2_GetComponentToWorld` _returnvalue)))))

(fn `SetUp spawn Points`
  (for _array_element (`self.Lane Position`)
    (for _index (range 2)
      (bind _returnvalue (`AddComponent|NODE_AddArrowComponent-0` :`RelativeTransform` (`KismetMathLibrary.MakeTransform` (`KismetMathLibrary.MakeVector` (* _index 650.0) _array_element))))
      (`KismetArrayLibrary.Array_Add` (`self.Spawn Points`) (`SceneComponent.K2_GetComponentToWorld` _returnvalue)))))

(fn `Spanw Coins`
  (locals (`random Spawn Points` :type "Array of Transform Structure"))
  (bind _output_get (set `local.random Spawn Points` (`self.CSpawn Points`)))
  (`KismetArrayLibrary.Array_Shuffle` _output_get)
  (for _index (range (+ (`KismetMathLibrary.RandomIntegerInRange` 3 5) 1))
    (switch `int` 0
      (:`0`
        (`AddComponent|NODE_AddChildActorComponent-7` :`RelativeTransform` (`KismetMathLibrary.MakeRelativeTransform` (`|GetArrayItem` (`local.random Spawn Points`) _index) (`self.GetTransform`)))))))

(fn `Spawn_Obstacles`
  (locals (`random Spawn Points` :type "Array of Transform Structure"))
  (bind _output_get (set `local.random Spawn Points` (`self.Spawn Points`)))
  (`KismetArrayLibrary.Array_Shuffle` _output_get)
  (for _index (range (+ (`KismetMathLibrary.RandomIntegerInRange` 0 1) 1))
    (switch `int` (`KismetMathLibrary.RandomIntegerInRange` 0 1)
      (:`0`
        (bind _returnvalue (`KismetMathLibrary.MakeRelativeTransform` (`|GetArrayItem` (`local.random Spawn Points`) _index) (`self.GetTransform`)))
        (`AddComponent|NODE_AddChildActorComponent-0` :`RelativeTransform` _returnvalue))
      (:`1`
        (`AddComponent|NODE_AddChildActorComponent-1` :`RelativeTransform` _returnvalue)))))

(fn `SpawnPowerUp`
  (locals (`random Spawn Points` :type "Array of Transform Structure"))
  (bind _asbp_runner_game_mode (cast `/Game/Runner/BluePrint/BP_RunnerGameMode` (`GameplayStatics.GetGameMode`)))
  (if (> (`/Game/Runner/BluePrint/BP_RunnerGameMode.FloorCount` _asbp_runner_game_mode) 5)
    (set `/Game/Runner/BluePrint/BP_RunnerGameMode.FloorCount` 0 _asbp_runner_game_mode)
    (bind _output_get (set `local.random Spawn Points` (`self.PSpawnPoints`)))
    (`KismetArrayLibrary.Array_Shuffle` _output_get)
    (`AddComponent|NODE_AddChildActorComponent-8` :`RelativeTransform` (`KismetMathLibrary.MakeRelativeTransform` (`|GetArrayItem` (`local.random Spawn Points`)) (`self.GetTransform`)))))

(fn `UserConstructionScript`
  (`self.SetUp spawn Points`)
  (`self.Spawn_Obstacles`)
  (`self.Coin Spawn Points`)
  (`self.Spanw Coins`)
  (`self.PowerUp_SpawnPoints`)
  (`self.SpawnPowerUp`))