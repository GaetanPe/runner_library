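; BP_FloorStart is a floor tile for the runner game, apparently the starting one, with a custom event for scattering coins.
; SpanwCoins copies and shuffles CSpawnPoints, then loops over a small random count, adding a child actor component at each picked point, converted relative to the tile's transform.
; BeginPlay, overlap and Tick are disabled stubs, the construction script is empty, and nothing here calls SpanwCoins.
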(event `Spanw Coins`
  (bind _output_get (set `self.random Spawn Points` (`self.CSpawn Points`)))
  (`KismetArrayLibrary.Array_Shuffle` _output_get)
  (for _index (range (+ (`KismetMathLibrary.RandomIntegerInRange` 3 5) 1))
    (switch `int` 0
      (:`0`
        (`AddComponent|NODE_AddChildActorComponent-7` :`RelativeTransform` (`KismetMathLibrary.MakeRelativeTransform` (`|GetArrayItem` (`self.random Spawn Points`) _index) (`self.GetTransform`)))))))

(fn `UserConstructionScript`)