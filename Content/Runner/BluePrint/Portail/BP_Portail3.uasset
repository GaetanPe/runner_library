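; BP_Portail3 is a runner portal that switches the game to universe 0 when the player character enters it.
; On overlap with the runner, it plays a camera shutter sound, sets LevelUniverse on BP_RunnerGameMode, resets the floor, prints a debug message and destroys itself.
; A second overlap branch destroys the portal if it touches a wall obstacle.
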(event `self.ReceiveActorBeginOverlap`
  (params (OtherActor :type "Actor Object Reference"))
  (`|ExecutionSequence`
    (:`then_0`
      (cast `/Game/Runner/BluePrint/Characters/Bp_RunnerCharacter` OtherActor)
      (bind _asbp_runner_game_mode (cast `/Game/Runner/BluePrint/BP_RunnerGameMode` (`GameplayStatics.GetGameMode`)))
      (`GameplayStatics.PlaySound2D` "/Engine/VREditor/Sounds/UI/Camera_Shutter.Camera_Shutter" 1.0 1.0 0.0 null null)
      (set `/Game/Runner/BluePrint/BP_RunnerGameMode.LevelUniverse` 0 _asbp_runner_game_mode)
      (`/Game/Runner/BluePrint/BP_RunnerGameMode.ResetFloor` _asbp_runner_game_mode)
      (`KismetSystemLibrary.PrintString` "On change de monde 0" true true (struct :`R` 0.027499 :`G` 1.0 :`B` 0.031178 :`A` 1.0))
      (`self.K2_DestroyActor`))
    (:`then_1`
      ;[1 1 1] Si le magnet est sur un obstacle on le supprime
      (cast `/Game/Runner/BluePrint/Obstacles/BP_Obstacles_Wall` OtherActor)
      (`self.K2_DestroyActor`))))

(fn `UserConstructionScript`)