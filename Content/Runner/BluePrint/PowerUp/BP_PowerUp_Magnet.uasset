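; Magnet power-up pickup for the runner game that sets the runner's IsMagnetActive flag for a duration taken from the game mode.
; On overlap it plays a sound and hides itself; if no magnet is active, it starts a debug-printed countdown in MagnetTimer.
; A parallel delay clears the flag and destroys the actor.
; It also destroys itself when overlapping walls, blockers, coins or Multi power-ups.
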(event `self.ReceiveActorBeginOverlap`
  (params (OtherActor :type "Actor Object Reference"))
  (`|ExecutionSequence`
    (:`then_0`
      (bind _asbp_runner_character (cast `/Game/Runner/BluePrint/Characters/Bp_RunnerCharacter` OtherActor))
      (bind _asbp_runner_game_mode (cast `/Game/Runner/BluePrint/BP_RunnerGameMode` (`GameplayStatics.GetGameMode`)))
      (`GameplayStatics.PlaySound2D` "/Engine/VREditor/Sounds/UI/Camera_Shutter.Camera_Shutter" 1.0 1.0 0.0 null null)
      (`self.SetActorHiddenInGame` true)
      (if (not (`/Game/Runner/BluePrint/Characters/Bp_RunnerCharacter.IsMagnetActive?` _asbp_runner_character))
        (set `/Game/Runner/BluePrint/Characters/Bp_RunnerCharacter.IsMagnetActive?` true _asbp_runner_character)
        (bind _magnettimermax (`/Game/Runner/BluePrint/BP_RunnerGameMode.MagnetTimerMax` _asbp_runner_game_mode))
        (bind _returnvalue (+ _magnettimermax 1.0))
        (set `/Game/Runner/BluePrint/BP_RunnerGameMode.MagnetTimer` _returnvalue _asbp_runner_game_mode)
        (`KismetSystemLibrary.PrintString` "magnet activate")
        (`|ExecutionSequence`
          (:`then_0`
            ;[1 1 1] juste pour afficher combien de temps il reste au magnet
            (`/Game/Runner/BluePrint/Inputs/ForLoopDelay.ForLoopWithDelay` 0 (`KismetMathLibrary.FTrunc` _returnvalue) 1.0
              (:`loop Body`
                (bind _result (`/Engine/EditorBlueprintResources/StandardMacros.DecrementFloat` (`/Game/Runner/BluePrint/BP_RunnerGameMode.MagnetTimer` _asbp_runner_game_mode))
                  (:`  `
                    (bind _output_get (set `/Game/Runner/BluePrint/BP_RunnerGameMode.MagnetTimer` (`KismetMathLibrary.FMax` _result) _asbp_runner_game_mode))
                    (`KismetSystemLibrary.PrintString` (`KismetStringLibrary.Conv_DoubleToString` _output_get) true true (struct :`R` 1.0 :`G` 0.23311 :`B` 0.876368 :`A` 1.0)))))))
          (:`then_1`
            ;[1 1 1] une fois la durée du magnet terminé, on le supprime et on met a jour le statut du Runner
            (`KismetSystemLibrary.Delay` (+ _magnettimermax 0.2))
            (bind _asbp_runner_character_2 (cast `/Game/Runner/BluePrint/Characters/Bp_RunnerCharacter` (`GameplayStatics.GetPlayerCharacter` 0)))
            (set `/Game/Runner/BluePrint/Characters/Bp_RunnerCharacter.IsMagnetActive?` false _asbp_runner_character_2)
            (`KismetSystemLibrary.PrintString` "magnet desactivate")
            (`self.K2_DestroyActor`)))))
    (:`then_1`
      ;[1 1 1] Si le magnet est sur un obstacle on le supprime
      (cast `/Game/Runner/BluePrint/Obstacles/BP_Obstacles_Wall` OtherActor)
      (`self.K2_DestroyActor`))
    (:`then_2`
      ;[1 1 1] Si le magnet est sur une piece on le supprime
      (cast `/Game/Runner/BluePrint/PowerUp/BP_Coin` OtherActor)
      (`self.K2_DestroyActor`))
    (:`then_3`
      ;[1 1 1] Si le magnet est sur un multi on le supprime
      (cast `/Game/Runner/BluePrint/PowerUp/BP_PowerUp_Multi` OtherActor)
      (`self.K2_DestroyActor`))
    (:`then_4`
      (cast `/Game/Runner/BluePrint/Obstacles/BP_Obstacles_Blocker` OtherActor)
      (`self.K2_DestroyActor`))))

(fn `UserConstructionScript`)