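; Game mode for an endless runner that builds the track and, on the RunnerBase level, loads saved coins and power-up durations at start.
; AddFloor chains tiles through attach points, choosing one of two universe floors and placing a portal tile every twentieth.
; ExtendFloor appends tiles and trims the oldest, while ResetFloor clears most tiles and rebuilds in the second universe.
; Magnet and multiplier timer limits scale with saved levels, creating missing save slots.
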(event `self.ReceiveBeginPlay`
  (set `self.CoinParty` 0)
  ;[1 1 1] Si on est dans le level run, on genere des tuiles
  (bind _returnvalue (`GameplayStatics.GetCurrentLevelName` true))
  (if (`KismetStringLibrary.EqualEqual_StrStr` _returnvalue "RunnerBase")
    (`self.MagnetTimeUpdate`)
    (`self.MultiTimeUpdate`)
    (for _ (range (`self.number_of_tiles`))
      (`self.Add floor`)
      ;[1 1 1] a mettre dans une fonction a part
      (bind _returnvalue_2 (`GameplayStatics.LoadGameFromSlot` "CoinValue"))
      (bind _asrunner_save_game (cast `/Game/Runner/BluePrint/Runner_SaveGame` _returnvalue_2))
      (set `self.Coins` (`/Game/Runner/BluePrint/Runner_SaveGame.CoinValue` _asrunner_save_game)))))

(fn `Add floor`
  (bind _floorattachpoint (`self.FloorAttachPoint`))
  ;[1 1 1] Toutes les 20 tuiles on crée une tuile portail
  (if (== (mod (`self.FloorCount`) 20) 19)
    (bind _returnvalue (`|SpawnActorFromClass` "/Game/Runner/BluePrint/Floor/BP_Floor_portail.BP_Floor_portail_C" _floorattachpoint "Undefined" "MultiplyWithRoot" null null))
    (bind _returnvalue_2 (`/Game/Runner/BluePrint/Floor/BP_Floor.Get AttachPoint` _returnvalue))
    (set `self.FloorAttachPoint` _returnvalue_2)
    (`KismetArrayLibrary.Array_Add` (`self.floorTiles`) _returnvalue)
    (bind _result (`/Engine/EditorBlueprintResources/StandardMacros.IncrementInt` (`self.FloorCount`))
      (:`  `
        (set `self.FloorCount` _result)))
    (else
      (switch `int` (`self.LevelUniverse`)
        (:`0`
          ;[1 1 1] tuile univers1
          (bind _returnvalue_3 (`|SpawnActorFromClass` "/Game/Runner/BluePrint/Floor/BP_Floor.BP_Floor_C" _floorattachpoint "Undefined" "MultiplyWithRoot" null null))
          (bind _returnvalue_4 (`/Game/Runner/BluePrint/Floor/BP_Floor.Get AttachPoint` _returnvalue_3))
          (set `self.FloorAttachPoint` _returnvalue_4)
          (`KismetArrayLibrary.Array_Add` (`self.floorTiles`) _returnvalue_3)
          (bind _result_2 (`/Engine/EditorBlueprintResources/StandardMacros.IncrementInt` (`self.FloorCount`))
            (:`  `
              (set `self.FloorCount` _result_2))))
        (:`1`
          ;[1 1 1] Tuiles Unvivers 2
          (bind _returnvalue_5 (`|SpawnActorFromClass` "/Game/Runner/BluePrint/Floor/BP_Floor2.BP_Floor2_C" _floorattachpoint "Undefined" "MultiplyWithRoot" null null))
          (bind _returnvalue_6 (`/Game/Runner/BluePrint/Floor/BP_Floor.Get AttachPoint` _returnvalue_5))
          (set `self.FloorAttachPoint` _returnvalue_6)
          (`KismetArrayLibrary.Array_Add` (`self.floorTiles`) _returnvalue_5)
          (bind _result_3 (`/Engine/EditorBlueprintResources/StandardMacros.IncrementInt` (`self.FloorCount`))
            (:`  `
              (set `self.FloorCount` _result_3))))))))

(fn `extend floor`
  (bind _floortiles (`self.floorTiles`))
  (bind _output (`|GetArrayItem` _floortiles))
  (`self.Add floor`)
  (if (> (`KismetArrayLibrary.Array_Length` (`self.floorTiles`)) (+ (`self.number_of_tiles`) 15))
    (`self.K2_DestroyActor` _output)
    (`KismetArrayLibrary.Array_RemoveItem` _floortiles _output)))

(fn `MagnetTimeUpdate`
  (bind _saver_sub_class_2 (`self.Saver Sub class 2`))
  (bind _returnvalue (`GameplayStatics.DoesSaveGameExist` "MagnetLevel"))
  (if _returnvalue
    (`KismetSystemLibrary.PrintString` "MagnetLevel existe")
    (bind _returnvalue_2 (`GameplayStatics.LoadGameFromSlot` "MagnetLevel"))
    (bind _output_get (set `self.Saver Sub class 2` _returnvalue_2))
    (bind _asrunner_save_game (cast `/Game/Runner/BluePrint/Runner_SaveGame` _output_get))
    (bind _output_get_2 (set `/Game/Runner/BluePrint/Runner_SaveGame.MagnetLevel` (`/Game/Runner/BluePrint/Runner_SaveGame.MagnetLevel` _asrunner_save_game) _asrunner_save_game))
    (`GameplayStatics.SaveGameToSlot` _saver_sub_class_2 "MagnetLevel")
    ;[1 1 1] Mise a jour du timer MAX par rapport au lv du magnet
    (bind _output_get_3 (set `self.MagnetTimerMax` (`KismetMathLibrary.Conv_IntToDouble` (* _output_get_2 5))))
    (`KismetSystemLibrary.PrintString` "Magnet Timer max2 = " true true (struct :`R` 1.0 :`G` 0.051568 :`B` 0.081415 :`A` 1.0))
    (`KismetSystemLibrary.PrintString` (`KismetStringLibrary.Conv_DoubleToString` _output_get_3) true true (struct :`R` 1.0 :`G` 0.051568 :`B` 0.081415 :`A` 1.0))
    (else
      (`KismetSystemLibrary.PrintString` "Magnet level n existe pas")
      (bind _returnvalue_3 (`GameplayStatics.CreateSaveGameObject` "/Game/Runner/BluePrint/Runner_SaveGame.Runner_SaveGame_C"))
      (bind _output_get_4 (set `self.Saver Sub class 2` _returnvalue_3))
      (bind _asrunner_save_game_2 (cast `/Game/Runner/BluePrint/Runner_SaveGame` _output_get_4))
      (bind _output_get_5 (set `/Game/Runner/BluePrint/Runner_SaveGame.MagnetLevel` (`/Game/Runner/BluePrint/Runner_SaveGame.MagnetLevel` _asrunner_save_game_2) _asrunner_save_game_2))
      (`GameplayStatics.SaveGameToSlot` _saver_sub_class_2 "MagnetLevel")
      (bind _output_get_6 (set `self.MagnetTimerMax` (`KismetMathLibrary.Conv_IntToDouble` (* _output_get_5 5))))
      (`KismetSystemLibrary.PrintString` "Magnet Timer max3 = " true true (struct :`R` 1.0 :`G` 0.051568 :`B` 0.081415 :`A` 1.0))
      (`KismetSystemLibrary.PrintString` (`KismetStringLibrary.Conv_DoubleToString` _output_get_6) true true (struct :`R` 1.0 :`G` 0.051568 :`B` 0.081415 :`A` 1.0)))))

(fn `MultiTimeUpdate`
  (bind _saver_sub_class_2 (`self.Saver Sub class 2`))
  (bind _returnvalue (`GameplayStatics.DoesSaveGameExist` "MultiLevel"))
  (if _returnvalue
    (`KismetSystemLibrary.PrintString` "MultiLevel existe")
    (bind _returnvalue_2 (`GameplayStatics.LoadGameFromSlot` "MultiLevel"))
    (bind _output_get (set `self.Saver Sub class 2` _returnvalue_2))
    (bind _asrunner_save_game (cast `/Game/Runner/BluePrint/Runner_SaveGame` _output_get))
    (bind _output_get_2 (set `/Game/Runner/BluePrint/Runner_SaveGame.MultiLevel` (`/Game/Runner/BluePrint/Runner_SaveGame.MultiLevel` _asrunner_save_game) _asrunner_save_game))
    (`GameplayStatics.SaveGameToSlot` _saver_sub_class_2 "MultiLevel")
    ;[1 1 1] Mise a jour du timer MAX par rapport au lv du magnet
    (bind _output_get_3 (set `self.MultiTimerMax` (`KismetMathLibrary.Conv_IntToDouble` (* _output_get_2 5))))
    (`KismetSystemLibrary.PrintString` "Multi Timer max = " true true (struct :`R` 1.0 :`G` 0.219669 :`B` 0.884786 :`A` 1.0) 5.0)
    (`KismetSystemLibrary.PrintString` (`KismetStringLibrary.Conv_DoubleToString` _output_get_3) true true (struct :`R` 0.91119 :`G` 0.174305 :`B` 1.0 :`A` 1.0) 5.0)
    (else
      (`KismetSystemLibrary.PrintString` "MultiLevel n existe pas")
      (bind _returnvalue_3 (`GameplayStatics.CreateSaveGameObject` "/Game/Runner/BluePrint/Runner_SaveGame.Runner_SaveGame_C"))
      (bind _output_get_4 (set `self.Saver Sub class 2` _returnvalue_3))
      (bind _asrunner_save_game_2 (cast `/Game/Runner/BluePrint/Runner_SaveGame` _output_get_4))
      (bind _output_get_5 (set `/Game/Runner/BluePrint/Runner_SaveGame.MultiLevel` (`/Game/Runner/BluePrint/Runner_SaveGame.MultiLevel` _asrunner_save_game_2) _asrunner_save_game_2))
      (`GameplayStatics.SaveGameToSlot` _saver_sub_class_2 "MultiLevel")
      (bind _output_get_6 (set `self.MultiTimerMax` (`KismetMathLibrary.Conv_IntToDouble` (* _output_get_5 5))))
      (`KismetSystemLibrary.PrintString` "Multi Timer max = " true true (struct :`R` 1.0 :`G` 0.171331 :`B` 0.922362 :`A` 1.0) 5.0)
      (`KismetSystemLibrary.PrintString` (`KismetStringLibrary.Conv_DoubleToString` _output_get_6) true true (struct :`R` 0.91697 :`G` 0.171506 :`B` 1.0 :`A` 1.0) 5.0))))

(fn `ResetFloor`
  (bind _floortiles (`self.floorTiles`))
  (bind _output (`|GetArrayItem` _floortiles 1))
  (bind _returnvalue (`/Game/Runner/BluePrint/Floor/BP_Floor.Get AttachPoint` (`|GetArrayItem` (`self.floorTiles`))))
  (set `self.FloorAttachPoint` _returnvalue)
  (for _ (range 3 (`KismetArrayLibrary.Array_Length` (`self.floorTiles`)))
    (`self.K2_DestroyActor` _output)
    (`KismetArrayLibrary.Array_RemoveItem` _floortiles _output)
    (set `self.number_of_tiles` (- (`self.number_of_tiles`) 1)))
  (for _ (range 1 16)
    (set `self.LevelUniverse` 1)
    (`self.Add floor`)))

(fn `UserConstructionScript`)