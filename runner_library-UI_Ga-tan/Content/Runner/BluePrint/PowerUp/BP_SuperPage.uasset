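; BP_SuperPage is a runner collectible that the player character picks up by touching its Coin component.
; On pickup it increments SuperPageCollected on BP_RunnerGameMode, prints the count, plays a sound, destroys itself, then calls UpdateSuperPage on the character.
; The same overlap event also destroys the page when it touches a wall obstacle or magnet power-up, removing pages placed on existing objects.
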(event `self.Coin.OnComponentBeginOverlap`
  (params (OverlappedComponent :type "PrimitiveComponent Object Reference") (OtherActor :type "Actor Object Reference") (OtherComp :type "PrimitiveComponent Object Reference") (OtherBodyIndex :type Integer) (bFromSweep :type Boolean) (SweepResult :type "HitResult Structure (by ref)"))
  (`|ExecutionSequence`
    (:`then_0`
      ;[1 1 1] On verifie que c'est bien un character qui touche la piece
      (bind _asbp_runner_character (cast `/Game/Runner/BluePrint/Characters/Bp_RunnerCharacter` OtherActor))
      ;[1 1 1] On met a jour le score de piece dans le BP_RunnerGameMode et on joue le son avant de detruire la piece
      (bind _asbp_runner_game_mode (cast `/Game/Runner/BluePrint/BP_RunnerGameMode` (`GameplayStatics.GetGameMode`)))
      (bind _result (`/Engine/EditorBlueprintResources/StandardMacros.IncrementInt` (`/Game/Runner/BluePrint/BP_RunnerGameMode.SuperPageCollected` _asbp_runner_game_mode))
        (:`  `
          (`KismetSystemLibrary.PrintString` (`KismetStringLibrary.Conv_IntToString` _result) true true (struct :`R` 0.805556 :`G` 1.0 :`B` 0.323593 :`A` 1.0))
          (`GameplayStatics.PlaySound2D` "/Game/Audio/SFX/coin-and-mone.coin-and-mone" 1.0 1.0 0.0 null null)
          (`self.K2_DestroyActor`)
          (`/Game/Runner/BluePrint/Characters/Bp_RunnerCharacter.UpdateSuperPage` _asbp_runner_character))))
    (:`then_1`
      ;[1 1 1] Si la piece se trouve sur un objet deja existant, on le supprime
      (cast `/Game/Runner/BluePrint/Obstacles/BP_Obstacles_Wall` OtherActor)
      (`self.K2_DestroyActor`))
    (:`then_2`
      (cast `/Game/Runner/BluePrint/PowerUp/BP_PowerUp_Magnet` OtherActor)
      (`self.K2_DestroyActor`))))

(fn `UserConstructionScript`)