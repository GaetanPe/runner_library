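; BP_Obstacles_Blocker is a runner-game obstacle that kills the player unless they slide through it.
; On actor overlap it casts the other actor to Bp_RunnerCharacter and calls Death when IsSliding is false.
; One second after that call it sets the game to unpaused; BeginPlay, Tick and the construction script add no logic of their own.
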(event `self.ReceiveActorBeginOverlap`
  (params (OtherActor :type "Actor Object Reference"))
  ;[1 1 1] Le joueur traverse l'obstacle et ne slide pas <==> le joueur meurt
  (bind _asbp_runner_character (cast `/Game/Runner/BluePrint/Characters/Bp_RunnerCharacter` OtherActor))
  (if (not (`/Game/Runner/BluePrint/Characters/Bp_RunnerCharacter.IsSliding` _asbp_runner_character))
    (`/Game/Runner/BluePrint/Characters/Bp_RunnerCharacter.Death` _asbp_runner_character)
    (`KismetSystemLibrary.Delay` 1.0)
    (`GameplayStatics.SetGamePaused` false)))

(fn `UserConstructionScript`
  (`parent.UserConstructionScript`))