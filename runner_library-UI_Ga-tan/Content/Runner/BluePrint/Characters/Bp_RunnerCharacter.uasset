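; Player character for a three-lane endless runner that constantly moves forward and can jump, slide or switch lanes.
; Enhanced Input and touch swipes drive these moves, with a timeline interpolating lane changes.
; Slides add a downward impulse and, when grounded and moving, play a montage while briefly disabling input and ignoring Destructible collision.
; Death ragdolls the mesh, shows game over and saves high score and coins from the game mode.
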(event `self.ReceiveBeginPlay`
  ;[1 1 1] Ajout UI Gameplay + ajout du bon mapping de touche (dont le tactile)
  (bind _asplayer_controller (cast `PlayerController` (`self.GetController`)))
  (bind _returnvalue (pcsubsystem `EnhancedInputLocalPlayerSubsystem` _asplayer_controller))
  (`/Engine/EditorBlueprintResources/StandardMacros.IsValid` _returnvalue
    (:`Is Valid`
      (`EnhancedInputSubsystemInterface.AddMappingContext` _returnvalue "/Game/Runner/BluePrint/Inputs/IMC_RunnerDefaut.IMC_RunnerDefaut" 0 (struct)))))

(event `EnhancedInput|/Game/Runner/BluePrint/Inputs/Jump_IA`
  (params (ActionValue :type Boolean) (ElapsedSeconds :type "Float (double-precision)") (TriggeredSeconds :type "Float (double-precision)") (InputAction :type "InputAction Object Reference" :default "/Game/Runner/BluePrint/Inputs/Jump_IA.Jump_IA"))
  ;[1 1 1] Saut
  (:`Triggered`
    (`self.Jump`)))

(event `self.ReceiveTick`
  (params (DeltaSeconds :type "Float (single-precision)"))
  ;[1 1 1] Ajout runneur infinie (on ajoute une impulsion au jour a chaque update)
  (`self.AddMovementInput` (`KismetMathLibrary.GetForwardVector` (`KismetMathLibrary.MakeRotator` 0.0 0.0 (.yaw (`self.GetControlRotation`))))))

(event `EnhancedInput|/Game/Runner/BluePrint/Inputs/Slide_IA`
  (params (ActionValue :type Boolean) (ElapsedSeconds :type "Float (double-precision)") (TriggeredSeconds :type "Float (double-precision)") (InputAction :type "InputAction Object Reference" :default "/Game/Runner/BluePrint/Inputs/Slide_IA.Slide_IA"))
  (bind _charactermovement (`self.CharacterMovement`))
  ;[1 1 1] Glissade
  (:`Triggered`
    (`CharacterMovementComponent.AddImpulse` (`self.CharacterMovement`) (0.0 0.0 -1000.0) true :!label _label)
    (if (and (> (`KismetMathLibrary.VSize` (`MovementComponent.Velocity` _charactermovement)) 60.0) (not (`NavMovementComponent.IsFalling` _charactermovement)))
      ;;[1 1 1] Pour etre sur qu'on ne lance pas l'animation deux fois glissade pendant la glissade
      (`/Engine/EditorBlueprintResources/StandardMacros.DoOnce` false :!label _label_2
        (:`Completed`
          (`self.DisableInput` null)
          (`PrimitiveComponent.SetCollisionResponseToChannel` (`self.CapsuleComponent`) "ECC_Destructible" "ECR_Ignore")
          (set `self.IsSliding` true)
          (`AnimInstance.Montage_Play` (`SkeletalMeshComponent.GetAnimInstance` (`self.Mesh`)) "/Game/Runner/Animation/Running_Slide_Retargeted_Montage.Running_Slide_Retargeted_Montage" 1.5 "MontageLength" 0.0 true)
          (`KismetSystemLibrary.Delay` 0.7)
          (`PrimitiveComponent.SetCollisionResponseToChannel` (`self.CapsuleComponent`) "ECC_Destructible" "ECR_Block")
          (`self.EnableInput` null)
          (set `self.IsSliding` false)
          (goto _label_2 :!via `Reset`))))))

(event `Slide Function`
  ;[1 1 1] Glissade
  ;;[0.1976 0.2304 1] Pour la version tactile
  (goto _label))

(event `Change_Lanes`
  (params (`Shift Lanes` :type Integer))
  ;[1 1 1] Change d'axe
  (set `self.Target Lane index` (`KismetMathLibrary.Clamp` (+ `Shift Lanes` (`self.Current Lane Index`)) 0 2))
  (set `self.Current Y Position` (.y (`self.K2_GetActorLocation`)))
  ;;[1 1 1] Changer la timeline change Lane pour une transition plus rapide
  (bind (_direction _change_lane) (`Timeline|Transition` :!via `PlayFromStart`)
    (:`Update`
      (`self.K2_SetActorLocation` (`KismetMathLibrary.MakeVector` (.x (`self.K2_GetActorLocation`)) (`KismetMathLibrary.Lerp` (`self.Current Y Position`) (`|GetArrayItem` (`self.Lane Position`) (`self.Target Lane index`)) _change_lane) (.z (`self.K2_GetActorLocation`)))))
    (:`Finished`
      (set `self.Current Lane Index` (`self.Target Lane index`)))))

(event `EnhancedInput|/Game/Runner/BluePrint/Inputs/Left_IA`
  (params (ActionValue :type Boolean) (ElapsedSeconds :type "Float (double-precision)") (TriggeredSeconds :type "Float (double-precision)") (InputAction :type "InputAction Object Reference" :default "/Game/Runner/BluePrint/Inputs/Left_IA.Left_IA"))
  ;[1 1 1] Change d'axe
  ;;[1 0.7536 0.3437] On va gauche on change de "lanes" idem a droite
  (:`Triggered`
    (`self.Change_Lanes` -1)))

(event `EnhancedInput|/Game/Runner/BluePrint/Inputs/Right_IA`
  (params (ActionValue :type Boolean) (ElapsedSeconds :type "Float (double-precision)") (TriggeredSeconds :type "Float (double-precision)") (InputAction :type "InputAction Object Reference" :default "/Game/Runner/BluePrint/Inputs/Right_IA.Right_IA"))
  ;[1 1 1] Change d'axe
  ;;[1 0.7536 0.3437] On va gauche on change de "lanes" idem a droite
  (:`Triggered`
    (`self.Change_Lanes` 1)))

(event `InputTouch`
  (params (Location :type "Vector Structure") (FingerIndex :type "ETouchIndex Enum"))
  (bind _returnvalue (`KismetMathLibrary.MakeVector2D` Location_X Location_Y))
  (bind (_returnvalue_x _returnvalue_y) (`KismetMathLibrary.BreakVector2D` (- (`self.Touch Start 2D`) (`self.Touch End 2D`))))
  (bind _returnvalue_x_2 (`KismetMathLibrary.BreakVector2D` (- (`self.Touch Start 2D`) (`self.Touch End 2D`))))
  (bind _returnvalue_x_3 (`KismetMathLibrary.BreakVector2D` (- (`self.Touch Start 2D`) (`self.Touch End 2D`))))
  (bind (_returnvalue_x_4 _returnvalue_y_2) (`KismetMathLibrary.BreakVector2D` (- (`self.Touch Start 2D`) (`self.Touch End 2D`))))
  ;[1 1 1] Input Mobile
  (:`Pressed`
    (set `self.Touch Start 2D` _returnvalue)
    (set `self.IsTrigged?` true))
  (:`Moved`
    (set `self.Touch End 2D` _returnvalue)
    (if (`self.IsTrigged?`)
      (`|ExecutionSequence`
        (:`then_0`
          (if (> _returnvalue_x_2 (`self.Move Amount`))
            (`self.Change_Lanes` -1)))
        (:`then_1`
          (if (< _returnvalue_x_3 (* (`self.Move Amount`) -1.0))
            (`self.Change_Lanes` 1)))
        (:`then_2`
          (if (> _returnvalue_y_2 (`self.Move Amount`))
            (`self.Jump`)))
        (:`then_3`
          (if (< _returnvalue_y (* (`self.Move Amount`) -1.0))
            (`self.Slide Function`)))))))

(fn `Death`
  ;[1 1 1] Le character meurt == pas d'input et de mouvement pour lui
  (`CharacterMovementComponent.DisableMovement` (`self.CharacterMovement`))
  (`self.DisableInput` null)
  (`PrimitiveComponent.SetSimulatePhysics` (`self.Mesh`) true)
  ;[1 1 1] On supprime tout les widget pour mettre celui du game over
  (`WidgetLayoutLibrary.RemoveAllWidgets`)
  (bind _returnvalue (`|CreateWidget` "/Game/BluePrint/UI/WBP_GameOver.WBP_GameOver_C"))
  (`UserWidget.AddToViewport` _returnvalue 0)
  (set `PlayerController.bShowMouseCursor` true (`GameplayStatics.GetPlayerController` 0))
  ;[1 1 1] On met a jour le score et le nombre de pieces collectées
  (`self.SaveHightScore`)
  (`self.UpdateCoinsDeath`))

(fn `SaveHightScore`
  ;[1 1 1] via le RunnerGamemode on checke le hightscore enregisté
  (bind _asbp_runner_game_mode (cast `/Game/Runner/BluePrint/BP_RunnerGameMode` (`GameplayStatics.GetGameMode`)))
  (bind _returnvalue (`GameplayStatics.DoesSaveGameExist` "HightScore"))
  (if _returnvalue
    (bind _returnvalue_2 (`GameplayStatics.LoadGameFromSlot` "HightScore"))
    (bind _output_get (set `self.Saver Sub Class` _returnvalue_2))
    (bind _asrunner_save_game (cast `/Game/Runner/BluePrint/Runner_SaveGame` _output_get))
    (bind _currentpoints (`/Game/Runner/BluePrint/BP_RunnerGameMode.CurrentPoints` _asbp_runner_game_mode))
    (if (> _currentpoints (`/Game/Runner/BluePrint/Runner_SaveGame.HightScore` _asrunner_save_game))
      (set `/Game/Runner/BluePrint/Runner_SaveGame.HightScore` _currentpoints _asrunner_save_game)
      (`GameplayStatics.SaveGameToSlot` (`self.Saver Sub Class`) "HightScore"))
    (else
      (bind _returnvalue_3 (`GameplayStatics.CreateSaveGameObject` "/Game/Runner/BluePrint/Runner_SaveGame.Runner_SaveGame_C"))
      (bind _output_get_2 (set `self.Saver Sub Class` _returnvalue_3))
      (bind _asrunner_save_game_2 (cast `/Game/Runner/BluePrint/Runner_SaveGame` _output_get_2))
      (set `/Game/Runner/BluePrint/Runner_SaveGame.HightScore` _currentpoints _asrunner_save_game_2)
      (`GameplayStatics.SaveGameToSlot` (`self.Saver Sub Class`) "HightScore"))))

(fn `UpdateCoins`
  ;[1 1 1] Meme principe qu'avec SaveHight Score sauf qu'ici cest pour les pieces colléctées
  (cast `/Game/Runner/BluePrint/BP_RunnerGameMode` (`GameplayStatics.GetGameMode`)))

(fn `UpdateCoinsDeath`
  ;[1 1 1] Meme principe qu'avec SaveHight Score sauf qu'ici cest pour les pieces colléctées
  (bind _asbp_runner_game_mode (cast `/Game/Runner/BluePrint/BP_RunnerGameMode` (`GameplayStatics.GetGameMode`)))
  (bind _returnvalue (`GameplayStatics.DoesSaveGameExist` "CoinValue"))
  (if _returnvalue
    (bind _returnvalue_2 (`GameplayStatics.LoadGameFromSlot` "CoinValue"))
    (bind _output_get (set `self.Saver Sub Class` _returnvalue_2))
    (bind _asrunner_save_game (cast `/Game/Runner/BluePrint/Runner_SaveGame` _output_get))
    (bind _returnvalue_3 (+ (`/Game/Runner/BluePrint/BP_RunnerGameMode.Coins` _asbp_runner_game_mode) (`/Game/Runner/BluePrint/BP_RunnerGameMode.CoinParty` _asbp_runner_game_mode)))
    (set `/Game/Runner/BluePrint/Runner_SaveGame.CoinValue` _returnvalue_3 _asrunner_save_game)
    (`GameplayStatics.SaveGameToSlot` (`self.Saver Sub Class`) "CoinValue")
    (else
      (bind _returnvalue_4 (`GameplayStatics.CreateSaveGameObject` "/Game/Runner/BluePrint/Runner_SaveGame.Runner_SaveGame_C"))
      (bind _output_get_2 (set `self.Saver Sub Class` _returnvalue_4))
      (bind _asrunner_save_game_2 (cast `/Game/Runner/BluePrint/Runner_SaveGame` _output_get_2))
      (set `/Game/Runner/BluePrint/Runner_SaveGame.CoinValue` _returnvalue_3 _asrunner_save_game_2)
      (`GameplayStatics.SaveGameToSlot` (`self.Saver Sub Class`) "CoinValue"))))

(fn `UpdateSuperPage`
  ;[1 1 1] Meme principe qu'avec SaveHight Score sauf qu'ici cest pour les pieces colléctées
  (bind _asbp_runner_game_mode (cast `/Game/Runner/BluePrint/BP_RunnerGameMode` (`GameplayStatics.GetGameMode`)))
  (bind _returnvalue (`GameplayStatics.DoesSaveGameExist` "SuperPage"))
  (if _returnvalue
    (bind _returnvalue_2 (`GameplayStatics.LoadGameFromSlot` "SuperPage"))
    (bind _output_get (set `self.Saver Sub Class` _returnvalue_2))
    (bind _asrunner_save_game (cast `/Game/Runner/BluePrint/Runner_SaveGame` _output_get))
    (bind _superpagecollected (`/Game/Runner/BluePrint/BP_RunnerGameMode.SuperPageCollected` _asbp_runner_game_mode))
    (set `/Game/Runner/BluePrint/Runner_SaveGame.SuperPage` _superpagecollected _asrunner_save_game)
    (`GameplayStatics.SaveGameToSlot` (`self.Saver Sub Class`) "Superpage")
    (else
      (bind _returnvalue_3 (`GameplayStatics.CreateSaveGameObject` "/Game/Runner/BluePrint/Runner_SaveGame.Runner_SaveGame_C"))
      (bind _output_get_2 (set `self.Saver Sub Class` _returnvalue_3))
      (bind _asrunner_save_game_2 (cast `/Game/Runner/BluePrint/Runner_SaveGame` _output_get_2))
      (set `/Game/Runner/BluePrint/Runner_SaveGame.SuperPage` _superpagecollected _asrunner_save_game_2)
      (`GameplayStatics.SaveGameToSlot` (`self.Saver Sub Class`) "Superpage"))))

(fn `UserConstructionScript`)